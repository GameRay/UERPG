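; Loot pickup actor that grants a random coin reward when a JLRPGCharacter overlaps it.
; On overlap it destroys itself, adds a BagWidget to the viewport and shows the mouse cursor.
; It then writes the random amount to AmountFound on JLGameMode and adds it to the first player character's Coins, regardless of which character triggered the overlap.
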(event `self.ReceiveActorBeginOverlap`
  (params (OtherActor :type "Actor Object Reference"))
  (cast `JLRPGCharacter` OtherActor)
  (`self.K2_DestroyActor`)
  (bind _returnvalue (`|CreateWidget` "/Game/Blueprint/BagWidget.BagWidget_C"))
  (`UserWidget.AddToViewport` _returnvalue 0)
  (set `PlayerController.bShowMouseCursor` true (`GameplayStatics.GetPlayerController` 0))
  (bind _asjlgame_mode (cast `/Game/ThirdPersonCPP/Blueprints/JLGameMode` (`GameplayStatics.GetGameMode`)))
  (bind _output_get (set `/Game/ThirdPersonCPP/Blueprints/JLGameMode.AmountFound` (`KismetMathLibrary.RandomIntegerInRange` 0 50) _asjlgame_mode))
  (bind _asjlrpgcharacter (cast `JLRPGCharacter` (`GameplayStatics.GetPlayerCharacter` 0)))
  (set `JLRPGCharacter.Coins` (+ _output_get (`JLRPGCharacter.Coins` _asjlrpgcharacter)) _asjlrpgcharacter))

(fn `UserConstructionScript`)