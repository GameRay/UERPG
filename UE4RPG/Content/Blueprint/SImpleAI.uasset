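; Simple enemy AI that patrols random navmesh points and moves to any player character its PawnSensing detects, then resumes patrol.
; Overlaps deal damage: Paladin axe hits count only during a skill, throttled by a cooldown, while WeaponItems explode and are destroyed.
; At zero health it plays a burst, spawns loot, destroys itself, then awards experience and saves through JLGameMode.
; TakeDamage only spawns a flame effect, without changing health.
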(event `self.ReceiveBeginPlay`
  (set `self.DamageCycle` 0.0))

(event `self.ReceiveActorBeginOverlap`
  (params (OtherActor :type "Actor Object Reference"))
  (bind _returnvalue (`KismetSystemLibrary.GetGameTimeInSeconds`))
  (bind _asweapon_axe (cast `/Game/Blueprint/Weapon_Axe` OtherActor)
    (:`then`
      (bind _asbp_jlrpgcharacter_paladin (cast `/Game/ThirdPersonCPP/Blueprints/BP_JLRPGCharacter_Paladin` (`self.GetAttachParentActor` _asweapon_axe)))
      (if (`/Game/ThirdPersonCPP/Blueprints/BP_JLRPGCharacter_Paladin.SkillState` _asbp_jlrpgcharacter_paladin)
        (if (> (- _returnvalue (`self.AttcckedTime`)) (`self.DamageCycle`))
          (set `self.DamageCycle` 10.0)
          (set `self.AttcckedTime` _returnvalue)
          (`KismetSystemLibrary.PrintString` "Hello----------")
          (bind _output_get (set `self.Health` (- (`self.Health`) 0.2)))
          (if (<= _output_get 0.0)
            (`GameplayStatics.SpawnEmitterAtLocation` "/Game/InfinityBladeEffects/Effects/FX_Mobile/Fire/combat/P_FireBall_Strong_MuzzFlash_01.P_FireBall_Strong_MuzzFlash_01" (`self.K2_GetActorLocation`))
            (`KismetSystemLibrary.Delay` 0.5)
            (`|SpawnActorFromClass` "/Game/Blueprint/LootPickUP.LootPickUP_C" (`self.GetTransform`) "Undefined" "OverrideRootScale" null null)
            (`self.K2_DestroyActor`)
            (bind _asjlgame_mode (cast `/Game/ThirdPersonCPP/Blueprints/JLGameMode` (`GameplayStatics.GetGameMode`)))
            (`/Game/ThirdPersonCPP/Blueprints/JLGameMode.AddExp` _asjlgame_mode 5)
            (`/Game/ThirdPersonCPP/Blueprints/JLGameMode.UpdateSaveGame` _asjlgame_mode)))))
    (:`CastFailed`
      (bind _asweapon_item (cast `/Game/Blueprint/WeaponItem` OtherActor))
      (bind _returnvalue_2 (`GameplayStatics.SpawnEmitterAtLocation` "/Game/InfinityBladeEffects/Effects/FX_Monsters/FX_Monster_Gruntling/Bomber/P_FireBombExplosion.P_FireBombExplosion" (`self.K2_GetActorLocation` _asweapon_item)))
      (`KismetSystemLibrary.Delay` 0.5)
      (`self.K2_DestroyActor` _asweapon_item)
      (`ActorComponent.K2_DestroyComponent` _returnvalue_2)
      (bind _output_get_2 (set `self.Health` (- (`self.Health`) 0.2)))
      (if (<= _output_get_2 0.0)
        (`GameplayStatics.SpawnEmitterAtLocation` "/Game/InfinityBladeEffects/Effects/FX_Mobile/Fire/combat/P_FireBall_Strong_MuzzFlash_01.P_FireBall_Strong_MuzzFlash_01" (`self.K2_GetActorLocation`))
        (`KismetSystemLibrary.Delay` 0.5)
        (`|SpawnActorFromClass` "/Game/Blueprint/LootPickUP.LootPickUP_C" (`self.GetTransform`) "Undefined" "OverrideRootScale" null null)
        (`self.K2_DestroyActor`)
        (bind _asjlgame_mode_2 (cast `/Game/ThirdPersonCPP/Blueprints/JLGameMode` (`GameplayStatics.GetGameMode`)))
        (`/Game/ThirdPersonCPP/Blueprints/JLGameMode.AddExp` _asjlgame_mode_2 5)
        (`/Game/ThirdPersonCPP/Blueprints/JLGameMode.UpdateSaveGame` _asjlgame_mode_2)))))

(event `self.PawnSensing.OnSeePawn`
  (params (Pawn :type "Pawn Object Reference"))
  (bind _asjlrpgcharacter (cast `JLRPGCharacter` Pawn))
  (set `self.IsPatrol` false)
  (`|AIMoveTo` self (0.0 0.0 0.0) _asjlrpgcharacter 1.0
    (:`OnSuccess`
      _)
    (:`OnFail`
      _))
  (set `self.IsPatrol` true))

(event `self.ReceiveTick`
  (params (DeltaSeconds :type "Float (single-precision)"))
  (if (`self.IsPatrol`) :!label _label
    (`KismetSystemLibrary.Delay` 3.0)
    (`|AIMoveTo` self (`NavigationSystemV1.K2_GetRandomLocationInNavigableRadius` (`self.K2_GetActorLocation`) 1000.0 null null) null 1.0 true
      (:`then`
        (goto _label)))))

(fn `TakeDamage`
  (`GameplayStatics.SpawnEmitterAtLocation` "/Game/InfinityBladeEffects/Effects/FX_Monsters/FX_Monster_Gruntling/FlameThrower/P_FlameExplode.P_FlameExplode" (`self.K2_GetActorLocation`)))

(fn `UserConstructionScript`)